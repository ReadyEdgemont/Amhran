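; AI controller Blueprint for NPC characters that starts their behavior tree on BeginPlay and handles combat notifications.
; Strike notifications run a single-target melee sweep using the equipped weapon's range and apply its damage to any hit.
; Other notifications toggle the pawn's parryable window and re-enable attacking when an attack ends.
; Death stops movement, behavior logic and the mesh, and disables capsule collision.
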(event `self.ReceiveBeginPlay`
  (bind _asnpc_character_bp (cast `/Game/Blueprints/NPCs/npcCharacterBP` (`self.K2_GetPawn`))
    (:`then`
      (set `self.Controlled_NPC_Character_BP` _asnpc_character_bp)
      (`self.RunBehaviorTree` "/Game/Blueprints/NPCs/npcAITree.npcAITree"))
    (:`CastFailed`
      (`KismetSystemLibrary.PrintString` "ERROR: Non-NPC Character controlled by AI Controller BP!") ; Error Message
    )))

(fn `NPC_AI_Can_Be_Parried`
  (returns (Parryable :type Boolean))
  (return (`CharacterPlus.CanBeParried` (`self.Controlled_NPC_Character_BP`))))

(fn `NPC_AI_Notified_Death`
  (`self.StopMovement`)
  (`BrainComponent.StopLogic` (`self.BrainComponent`) "Died")
  (bind _asnpc_character_bp (cast `/Game/Blueprints/NPCs/npcCharacterBP` (`self.K2_GetPawn`))
    (:`then`
      (`SkeletalMeshComponent.Stop` (`Character.Mesh` _asnpc_character_bp))
      (`PrimitiveComponent.SetCollisionEnabled` (`Character.CapsuleComponent` _asnpc_character_bp) "NoCollision"))
    (:`CastFailed`
      (`KismetSystemLibrary.PrintString` "Error: Failed to cast pawn to npcCharacter_BP is NPC_AI_Notified_Death!"))))

(fn `NPC_AI_Notified_Parryable_Enter`
  (set `CharacterPlus.CanBeParried` true (`self.Controlled_NPC_Character_BP`)))

(fn `NPC_AI_Notified_parryable_Exit`
  (set `CharacterPlus.CanBeParried` false (`self.Controlled_NPC_Character_BP`)))

(fn `NPC_AI_Notified_Strike`
  (returns (DidHit :type Boolean))
  (bind _asnpc_character (cast `npcCharacter` (`self.K2_GetPawn`))
    (:`then`
      (bind _returnvalue (`CharacterPlus.GetEquippedWeapon` _asnpc_character))
      (bind _returnvalue_2 (`CombatLibrary.MeleeAttackCheckSingle` (`Weapon.Range` _returnvalue) 30.0 _asnpc_character))
      (if (`KismetSystemLibrary.IsValid` _returnvalue_2)
        (`CharacterPlus.Damage` _returnvalue_2 (`Weapon.Damage` _returnvalue))
        (return true)
        (else
          (return false))))
    (:`CastFailed`
      (`KismetSystemLibrary.PrintString` "ERROR: Pawn notified of strike is not an npcCharacter!")
      (return false))))

(fn `NPC_AI_Notify_Attack_End`
  (set `CharacterPlus.CanAttack` true (`self.Controlled_NPC_Character_BP`)))

(fn `UserConstructionScript`)