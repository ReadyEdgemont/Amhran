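; NPC character Blueprint that relays parry and death notifications to the NPC's animation and AI.
; A parry notification clears CanBeParried and forwards to the TPP_Anim instance, only while that flag is set.
; A death notification forwards to the npcAI_BP controller, and failed casts in either path print errors.
; BeginPlay, the construction script and FoundEnemy are empty.
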(event `self.ReceiveBeginPlay`)

(event `self.CharacterPlusNotifiedParried`
  ;[1 1 1] Notify Parried
  (bind _astpp_anim (cast `/Game/Blueprints/NPCs/Animation/TPP_Anim` (`SkeletalMeshComponent.GetAnimInstance` (`self.Mesh`)))
    (:`then`
      (if (`self.CanBeParried`)
        (set `self.CanBeParried` false)
        (`/Game/Blueprints/NPCs/Animation/TPP_Anim.Notified_Parried` _astpp_anim)))
    (:`CastFailed`
      (`KismetSystemLibrary.PrintString` "ERROR: Invalid animation instance on a notified parry NPC!") ; Error Message
    )))

(event `self.CharacterPlusNotifiedDeath`
  ;[1 1 1] Notify Death
  (bind _returnvalue (`AIBlueprintHelperLibrary.GetAIController` self))
  (bind _asnpc_ai_bp (cast `/Game/Blueprints/NPCs/npcAI_BP` _returnvalue)
    (:`then`
      (`/Game/Blueprints/NPCs/npcAI_BP.NPC_AI_Notified_Death` _asnpc_ai_bp))
    (:`CastFailed`
      (`KismetSystemLibrary.PrintString` "ERROR: Failed to cast AI Controller to NPC_AI_BP to notify of death!"))))

(fn `FoundEnemy`
  (params (Enemy :type "CharacterPlus Object Reference")))

(fn `UserConstructionScript`)