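; BP_Amhran_Player is the player Blueprint that sets up the in-game HUD and opens the pause menu.
; On BeginPlay it creates the HUD widget, adds it to the viewport and restores game-only input after the menus.
; Escape creates the pause widget if none is valid, then uses BP_AmhranPlayerController to switch to UI-only input, center and show the cursor, and pause the game.
; A failed controller cast prints an error.
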(event `self.ReceiveBeginPlay`
  ;[1 1 1] Create HUD
  (bind _returnvalue (`|CreateWidget` "/Game/Blueprints/Menus/HUD/HUD.HUD_C"))
  (bind _output_get (set `self.HUD` _returnvalue))
  (`UserWidget.AddToViewport` _output_get 0)
  (`WidgetBlueprintLibrary.SetInputMode_GameOnly` (`GameplayStatics.GetPlayerController` 0)) ; Clear the cursor from the screen after the menus are done
)

(event `self.ReceiveTick`
  (params (DeltaSeconds :type "Float (single-precision)")))

(event `Key|Escape`
  (params (Key :type "Key Structure" :default "AnyKey"))
  (bind _pausemenu (`self.PauseMenu`))
  (:`Pressed`
    (`/Engine/EditorBlueprintResources/StandardMacros.IsValid` _pausemenu
      (:`Is Valid`
        _)
      (:`Is Not Valid`
        (bind _returnvalue (`|CreateWidget` "/Game/Blueprints/Menus/Pause/Pause.Pause_C"))
        (set `self.PauseMenu` _returnvalue)))
    (bind _asbp_amhran_player_controller (cast `/Game/Blueprints/Player/BP_AmhranPlayerController` (`GameplayStatics.GetPlayerController` 0))
      (:`then`
        (`WidgetBlueprintLibrary.SetInputMode_UIOnlyEx` _asbp_amhran_player_controller _pausemenu)
        (`UserWidget.AddToViewport` _pausemenu 0)
        (`AmhranPlayerController.CenterMouse` _asbp_amhran_player_controller)
        (set `PlayerController.bShowMouseCursor` true _asbp_amhran_player_controller)
        (`GameplayStatics.SetGamePaused` true))
      (:`CastFailed`
        (`KismetSystemLibrary.PrintString` "ERROR: Invalid Player Controller in BP_Amhran_Player!!!")))))

(fn `UserConstructionScript`)